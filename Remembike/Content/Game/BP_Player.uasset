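; BP_Player is the player Blueprint for a 2021 game jam project, relaying collision events to BP_GameJam2021PlayerController.
; A hit against a component named exactly "Building" calls OnStunned on the controller.
; Any actor overlap prints a debug string and passes the other actor to the controller's OnOverlap.
; The responses themselves live in the controller; BeginPlay, Tick and the construction script are empty.
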(event EventBeginPlay)

(event Collision|EventHit
  (params (MyComp :type Primitive%20Component%20Object%20Reference) (Other :type Actor%20Object%20Reference) (OtherComp :type Primitive%20Component%20Object%20Reference) (bSelfMoved :type Boolean) (HitLocation :type Vector :default "0, 0, 0") (HitNormal :type Vector :default "0, 0, 0") (NormalImpulse :type Vector :default "0, 0, 0") (Hit :type Hit%20Result%20Structure%20%28by%20ref%29))
  (if (Utilities|Enum|Equal(Enum) (Utilities|GetObjectName OtherComp) "Building")
    (bind _asbp_game_jam_2021player_controller (Utilities|Casting|CastToBP_GameJam2021PlayerController (Pawn|GetController self)))
    (Class|GameJam2021PlayerController|OnStunned _asbp_game_jam_2021player_controller)))

(event EventTick
  (params (DeltaSeconds :type Float%20%28single-precision%29)))

(event Collision|EventActorBeginOverlap
  (params (OtherActor :type Actor%20Object%20Reference))
  (Development|PrintString "OnOverlapFromBP")
  (bind _asbp_game_jam_2021player_controller (Utilities|Casting|CastToBP_GameJam2021PlayerController (Pawn|GetController self)))
  (Class|GameJam2021PlayerController|OnOverlap _asbp_game_jam_2021player_controller OtherActor))

(fn ConstructionScript)