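; Building actor that randomly populates its surroundings with elderly characters when play begins.
; On BeginPlay, an independent coin flip for each of twelve hardcoded offsets from the actor's location decides whether a character spawns there.
; BP_Granny can appear at the corners and edge midpoints of a square around the building, and BP_OldMan at four points between them.
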(event EventBeginPlay
  (bind _returnvalue (Transformation|GetActorLocation))
  (if (Math|Random|RandomBool)
    (Game|SpawnActorfromClass "/Game/Game/BP_Granny.BP_Granny_C" (Math|Transform|MakeTransform (+ _returnvalue "-800.000000,-800.000000,0.000000")) "Undefined" 0 0))
  (if (Math|Random|RandomBool)
    (Game|SpawnActorfromClass "/Game/Game/BP_Granny.BP_Granny_C" (Math|Transform|MakeTransform (+ _returnvalue "-800.000000,800.000000,0.000000")) "Undefined" 0 0))
  (if (Math|Random|RandomBool)
    (Game|SpawnActorfromClass "/Game/Game/BP_Granny.BP_Granny_C" (Math|Transform|MakeTransform (+ _returnvalue "800.000000,-800.000000,0.000000")) "Undefined" 0 0))
  (if (Math|Random|RandomBool)
    (Game|SpawnActorfromClass "/Game/Game/BP_Granny.BP_Granny_C" (Math|Transform|MakeTransform (+ _returnvalue "800.000000,800.000000,0.000000")) "Undefined" 0 0))
  (if (Math|Random|RandomBool)
    (Game|SpawnActorfromClass "/Game/Game/BP_Granny.BP_Granny_C" (Math|Transform|MakeTransform (+ _returnvalue "0.000000,800.000000,0.000000")) "Undefined" 0 0))
  (if (Math|Random|RandomBool)
    (Game|SpawnActorfromClass "/Game/Game/BP_Granny.BP_Granny_C" (Math|Transform|MakeTransform (+ _returnvalue "0.000000,-800.000000,0.000000")) "Undefined" 0 0))
  (if (Math|Random|RandomBool)
    (Game|SpawnActorfromClass "/Game/Game/BP_Granny.BP_Granny_C" (Math|Transform|MakeTransform (+ _returnvalue "-800.000000,0.000000,0.000000")) "Undefined" 0 0))
  (if (Math|Random|RandomBool)
    (Game|SpawnActorfromClass "/Game/Game/BP_Granny.BP_Granny_C" (Math|Transform|MakeTransform (+ _returnvalue "800.000000,0.000000,0.000000")) "Undefined" 0 0))
  (if (Math|Random|RandomBool)
    (Game|SpawnActorfromClass "/Game/Game/BP_OldMan.BP_OldMan_C" (Math|Transform|MakeTransform (+ _returnvalue "400.000000,800.000000,0.000000")) "Undefined" 0 0))
  (if (Math|Random|RandomBool)
    (Game|SpawnActorfromClass "/Game/Game/BP_OldMan.BP_OldMan_C" (Math|Transform|MakeTransform (+ _returnvalue "-400.000000,-800.000000,0.000000")) "Undefined" 0 0))
  (if (Math|Random|RandomBool)
    (Game|SpawnActorfromClass "/Game/Game/BP_OldMan.BP_OldMan_C" (Math|Transform|MakeTransform (+ _returnvalue "-800.000000,-400.000000,0.000000")) "Undefined" 0 0))
  (if (Math|Random|RandomBool)
    (Game|SpawnActorfromClass "/Game/Game/BP_OldMan.BP_OldMan_C" (Math|Transform|MakeTransform (+ _returnvalue "800.000000,400.000000,0.000000")) "Undefined" 0 0)))

(event Collision|EventActorBeginOverlap
  (params (OtherActor :type Actor%20Object%20Reference)))

(event EventTick
  (params (DeltaSeconds :type Float%20%28single-precision%29)))

(fn ConstructionScript)