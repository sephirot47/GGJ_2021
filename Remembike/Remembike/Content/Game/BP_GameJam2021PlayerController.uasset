(event EventBeginPlay
  (bind _returnvalue (Game|GetPlayerController 0))
  (bind _returnvalue_2 (UserInterface|CreateWidget "/Game/Game/WG_ArrowsHBox.WG_ArrowsHBox_C" _returnvalue))
  (bind _output_get (Variables|Default|SetArrowsWidget _returnvalue_2))
  (UserInterface|Viewport|AddtoViewport _output_get 0)
  (bind _returnvalue_3 (UserInterface|CreateWidget "/Game/Game/WG_HUD.WG_HUD_C" _returnvalue))
  (bind _output_get_2 (Variables|Default|SetHUDWidget _returnvalue_3))
  (UserInterface|Viewport|AddtoViewport _output_get_2 0)
  (bind _returnvalue_4 (UserInterface|CreateWidget "/Game/Game/WG_ThankDelivery.WG_ThankDelivery_C" _returnvalue))
  (bind _output_get_3 (Variables|Default|SetThankDeliveryWidget _returnvalue_4))
  (UserInterface|Viewport|AddtoViewport _output_get_3 0)
  (Widget|SetVisibility _output_get_3 "Hidden")
  (bind _returnvalue_5 (UserInterface|CreateWidget "/Game/Game/WG_PauseMenu.WG_PauseMenu_C" _returnvalue))
  (bind _output_get_4 (Variables|Default|SetPauseMenuWidget _returnvalue_5))
  (UserInterface|Viewport|AddtoViewport _output_get_4 0)
  (Widget|SetVisibility _output_get_4 "Hidden")
  (bind _asbp_game_instance (Utilities|Casting|CastToBP_GameInstance (Game|GetGameInstance)))
  (Default|StopMenuMusic _asbp_game_instance)
  (Audio|PlaySound2D "/Game/Game/Game_Music_Cue.Game_Music_Cue" 1.0 1.0 0.0 0 0))

(event EventSetScore
  (params (inScore :type Float%20%28single-precision%29))
  (bind _returnvalue (Math|Float|Floor inScore))
  (bind _asbp_game_instance (Utilities|Casting|CastToBP_GameInstance (Game|GetGameInstance)))
  (Variables|/Game/BP_GameInstance.BP_GameInstance_C|SetScore _asbp_game_instance _returnvalue)
  (Rendering|Components|TextRender|SetText (Variables|/Game/Game/WG_HUD.WG_HUD_C|GetText_Score (Variables|Default|GetHUDWidget)) (Utilities|Text|ToText(String) (Utilities|String|ToString(Integer) _returnvalue))))

(event EventShowThankDelivery
  (bind _thankdeliverywidget (Variables|Default|GetThankDeliveryWidget))
  (Widget|SetVisibility _thankdeliverywidget "Visible")
  (Utilities|Time|SetTimerbyFunctionName self "HideThankDelivery" 1.5)
  (Audio|PlaySound2D "/Game/Game/Delivery_Sound.Delivery_Sound" 1.0 1.0 0.0 0 0)
  (Default|OnShown _thankdeliverywidget))

(event EventOnPausePressedBP
  (bind _pausemenuwidget (Variables|Default|GetPauseMenuWidget))
  (Game|SetGamePaused (not (Game|IsGamePaused)))
  (if (Game|IsGamePaused)
    (Widget|SetVisibility _pausemenuwidget "Visible")
    (Variables|Default|SetbShowMouseCursor true)
    (else
      (Widget|SetVisibility _pausemenuwidget "Hidden")
      (Variables|Default|SetbShowMouseCursor false))))

(event EventSetAnimationRate
  (params (inAnimationRate :type Float%20%28single-precision%29))
  (bind _asbp_player (Utilities|Casting|CastToBP_Player (Game|Player|GetPlayerPawn 0)))
  (Components|Timeline|SetPlayRate (Variables|/Game/Game/BP_Player.BP_Player_C|GetPaperFlipbook _asbp_player) inAnimationRate))

(event EventShowDirectionArrows
  (params (directions :type Array%20of%20Integers))
  (CallFunction|ShowDirectionArrowsBP directions))

(event EventGotoLoseScreen
  (Game|OpenLevel(byObjectReference) "/Game/LoseScreen/LoseScreen.LoseScreen"))

(event EventSetDirectionArrowsOpacity
  (params (inOpacity :type Float%20%28single-precision%29))
  (CallFunction|SetDirectionArrowsOpacityBP inOpacity))

(event EventSetRemainingTime
  (params (inRemainingTime :type Float%20%28single-precision%29))
  (bind _returnvalue (Math|Float|Floor inRemainingTime))
  (bind _hudwidget (Variables|Default|GetHUDWidget))
  (bind _returnvalue_2 (Math|Integer|Max(Integer) _returnvalue))
  (bind _text_time (Variables|/Game/Game/WG_HUD.WG_HUD_C|GetText_Time _hudwidget))
  (Rendering|Components|TextRender|SetText _text_time (Utilities|Text|ToText(String) (Utilities|String|ToString(Integer) _returnvalue_2)))
  (if (< _returnvalue_2 10)
    (Class|TextBlock|SetFont _text_time (Utilities|Struct|MakeSlateFontInfo "/Engine/EngineFonts/Roboto.Roboto" 0 "(OutlineSize=0,bSeparateFillAlpha=False,bApplyOutlineToDropShadows=False,OutlineMaterial=None,OutlineColor=(R=0.000000,G=0.000000,B=0.000000,A=1.000000))" "Bold" 200))
    (Appearance|SetColorandOpacity _text_time (Utilities|Struct|MakeSlateColor "(R=1.000000,G=0.000000,B=0.000000,A=1.000000)") :!class /Script/UMG.TextBlock)
    (elif (< _returnvalue_2 20)
      (Class|TextBlock|SetFont _text_time (Utilities|Struct|MakeSlateFontInfo "/Engine/EngineFonts/Roboto.Roboto" 0 "(OutlineSize=0,bSeparateFillAlpha=False,bApplyOutlineToDropShadows=False,OutlineMaterial=None,OutlineColor=(R=0.000000,G=0.000000,B=0.000000,A=1.000000))" "Bold" 100))
      (Appearance|SetColorandOpacity _text_time (Utilities|Struct|MakeSlateColor "(R=1.000000,G=1.000000,B=0.000000,A=1.000000)") :!class /Script/UMG.TextBlock)
      (else
        (Class|TextBlock|SetFont _text_time (Utilities|Struct|MakeSlateFontInfo "/Engine/EngineFonts/Roboto.Roboto" 0 "(OutlineSize=0,bSeparateFillAlpha=False,bApplyOutlineToDropShadows=False,OutlineMaterial=None,OutlineColor=(R=0.000000,G=0.000000,B=0.000000,A=1.000000))" "Bold" 75))
        (Appearance|SetColorandOpacity _text_time (Utilities|Struct|MakeSlateColor "(R=1.000000,G=1.000000,B=1.000000,A=1.000000)") :!class /Script/UMG.TextBlock)))))

(event Input|ActionEvents|InputActionRing
  (params (Key :type Key%20Structure :default "None"))
  (:Pressed
    (Audio|PlaySound2D "/Game/Game/Ring_Cue.Ring_Cue" 1.0 1.0 0.0 0 0)))

(fn ConstructionScript)

(fn ShowDirectionArrowsBP
  (params (Directions :type Array%20of%20Integers))
  (bind _arrowswidget (Variables|Default|GetArrowsWidget))
  (bind _horizontalbox_0 (Variables|/Game/Game/WG_ArrowsHBox.WG_ArrowsHBox_C|GetHorizontalBox_0 _arrowswidget))
  (Widget|SetRenderOpacity _arrowswidget 1.0)
  (Widget|SetVisibility _arrowswidget "Visible")
  (Widget|Panel|ClearChildren _horizontalbox_0)
  (for _array_element Directions
    (switch int _array_element
      (:1
        (bind _returnvalue (UserInterface|CreateWidget "/Game/Game/WG_ArrowForward.WG_ArrowForward_C"))
        (Class|HorizontalBox|AddChildtoHorizontalBox _horizontalbox_0 _returnvalue))
      (:2
        (bind _returnvalue_2 (UserInterface|CreateWidget "/Game/Game/WG_ArrowLeft.WG_ArrowLeft_C"))
        (Class|HorizontalBox|AddChildtoHorizontalBox _horizontalbox_0 _returnvalue_2))
      (:3
        (bind _returnvalue_3 (UserInterface|CreateWidget "/Game/Game/WG_ArrowRight.WG_ArrowRight_C"))
        (Class|HorizontalBox|AddChildtoHorizontalBox _horizontalbox_0 _returnvalue_3)))))

(fn HideDirectionArrowsBP
  (Widget|SetVisibility (Variables|Default|GetArrowsWidget) "Hidden"))

(fn SetDirectionArrowsOpacityBP
  (params (Opacity :type Float%20%28single-precision%29))
  (Widget|SetRenderOpacity (Variables|Default|GetArrowsWidget) Opacity))

(fn HideThankDelivery
  (Widget|SetVisibility (Variables|Default|GetThankDeliveryWidget) "Hidden"))