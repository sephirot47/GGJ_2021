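; BP_Barrier is a barrier actor dressed with three trees that vary in size and proportion each time play begins.
; On BeginPlay it gives each of the three tree scene components a random relative scale, rolled independently per axis within a shrunken range, so scaling is non-uniform.
; It has no other active logic: the construction script is empty and the overlap and tick events are unused.
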(event EventBeginPlay
  (bind _returnvalue (Math|Random|RandomFloatinRange 0.5 0.9))
  (bind _returnvalue_2 (Math|Random|RandomFloatinRange 0.5 0.9))
  (bind _returnvalue_3 (Math|Random|RandomFloatinRange 0.5 0.9))
  (Transformation|SetRelativeScale3D (Variables|Default|GetTree0Scene) (Math|Vector|MakeVector _returnvalue_2 _returnvalue_2 _returnvalue_2))
  (Transformation|SetRelativeScale3D (Variables|Default|GetTree1Scene) (Math|Vector|MakeVector _returnvalue_3 _returnvalue_3 _returnvalue_3))
  (Transformation|SetRelativeScale3D (Variables|Default|GetTree2Scene) (Math|Vector|MakeVector _returnvalue _returnvalue _returnvalue)))

(event Collision|EventActorBeginOverlap
  (params (OtherActor :type Actor%20Object%20Reference)))

(event EventTick
  (params (DeltaSeconds :type Float%20%28single-precision%29)))

(fn ConstructionScript)