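; BP_GrannyController is a controller that makes its possessed pawn pace back and forth along a straight line.
; On BeginPlay it picks a random speed, reversal period and one of four axis directions, then Tick feeds that direction in as movement input.
; A looping timer flips the direction and mirrors the BP_Granny's RotationComp on its X scale to turn it around visually.
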(event EventBeginPlay
  (Variables|Default|SetSpeed (Math|Random|RandomFloatinRange 0.1 0.5))
  (bind _output_get (Variables|Default|SetPeriod (Math|Random|RandomFloatinRange 1.0 3.0)))
  (Utilities|Time|SetTimerbyFunctionName 0 "MoveInOppositeDirection" _output_get true)
  (switch int (Math|Random|RandomIntegerinRange 0 3)
    (:0
      (Variables|Default|SetMoveDir "1.000000, 0, 0"))
    (:1
      (Variables|Default|SetMoveDir "-1.000000, 0, 0"))
    (:2
      (Variables|Default|SetMoveDir "0.000000,1.000000, 0"))
    (:3
      (Variables|Default|SetMoveDir "0.000000,-1.000000, 0"))))

(event EventTick
  (params (DeltaSeconds :type Float%20%28single-precision%29))
  (Pawn|Input|AddMovementInput (Pawn|GetControlledPawn) (Variables|Default|GetMoveDir) (Variables|Default|GetSpeed) false))

(fn ConstructionScript)

(fn MoveinOppositeDirection
  (Variables|Default|SetMoveDir (* (Variables|Default|GetMoveDir) -1.0))
  (bind _asbp_granny (Utilities|Casting|CastToBP_Granny (Pawn|GetControlledPawn)))
  (Transformation|SetRelativeScale3D (Variables|/Game/Game/BP_Granny.BP_Granny_C|GetRotationComp _asbp_granny) (Math|Vector|MakeVector (* (.X (Math|Vector|BreakVector (Variables|/Script/Engine.SceneComponent|GetRelativeScale3D (Variables|/Game/Game/BP_Granny.BP_Granny_C|GetRotationComp _asbp_granny)))) -1.0) (.Y (Math|Vector|BreakVector (Variables|/Script/Engine.SceneComponent|GetRelativeScale3D (Variables|/Game/Game/BP_Granny.BP_Granny_C|GetRotationComp _asbp_granny)))) (.Z (Math|Vector|BreakVector (Variables|/Script/Engine.SceneComponent|GetRelativeScale3D (Variables|/Game/Game/BP_Granny.BP_Granny_C|GetRotationComp _asbp_granny)))))))